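; Grabbable component that tracks the grab state of a component on its owning actor and fires grab and release events.
; Grabbing stores the grab point as offsets from the owner's location and rotation, and seeds a target transform that callers update while held.
; It moves nothing in this graph; Tick only draws optional debug spheres, axes and an arrow from grab point to target.
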(event `self.ReceiveTick`
  (params (DeltaSeconds :type "Float (single-precision)"))
  (bind _targetlocation (`self.TargetLocation`))
  (bind _returnvalue (+ (`self.GrabLocationLocalSpace`) (`Actor.K2_GetActorLocation` (`self.GetOwner`))))
  (if (`self.DrawDebug`)
    (if (`self.Grabbed`)
      (`KismetSystemLibrary.DrawDebugSphere` _returnvalue 5.0 12 (struct :`R` 1.0 :`G` 0.017256 :`A` 1.0))
      (`KismetSystemLibrary.DrawDebugCoordinateSystem` _returnvalue (`self.GrabRotationLocalSpace`) 2.0)
      (`KismetSystemLibrary.DrawDebugSphere` _targetlocation 5.0 12 (struct :`G` 1.0 :`B` 0.240729 :`A` 1.0))
      (`KismetSystemLibrary.DrawDebugCoordinateSystem` _targetlocation (`self.TargetRotation`) 2.0)
      (`KismetSystemLibrary.DrawDebugArrow` _returnvalue _targetlocation 3.0))))

(fn `GrabComponent`
  (params (OverlappedComponent :type "PrimitiveComponent Object Reference") (GrabLocation :type "Vector Structure") (GrabRotation :type "Rotator Structure"))
  (returns (Grabbed :type Boolean))
  (bind _returnvalue (`self.GetOwner`))
  (if (and (not (`self.Grabbed`)) (== (`self.Component`) OverlappedComponent))
    (set `self.GrabLocationLocalSpace` (- GrabLocation (`Actor.K2_GetActorLocation` _returnvalue)))
    (set `self.GrabRotationLocalSpace` (`KismetMathLibrary.ComposeRotators` GrabRotation (`KismetMathLibrary.NegateRotator` (`Actor.K2_GetActorRotation` _returnvalue))))
    (set `self.TargetLocation` (`local.GrabLocation`))
    (set `self.TargetRotation` (`local.GrabRotation`))
    (set `self.Grabbed` true)
    (`self.OnGrab`)
    (return true)
    (else
      (return false))))

(fn `ReleaseComponent`
  (params (Component :type "Object Object Reference"))
  (if (and (== Component (`self.Component`)) (`self.Grabbed`))
    (set `self.Grabbed` false)
    (`self.OnRelease`)))

(fn `SetTargetPosition`
  (params (Component :type "PrimitiveComponent Object Reference") (Location :type "Vector Structure") (Rotation :type "Rotator Structure"))
  (if (and (`self.Grabbed`) (== Component (`self.Component`)))
    (set `self.TargetLocation` Location)
    (set `self.TargetRotation` Rotation)))