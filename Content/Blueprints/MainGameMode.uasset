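; Game mode for a broom-flying match with a score target and a catchable Snitch, running the timer, score and win/lose outcome.
; Restart seeds game state from game instance settings, and Tick counts down, firing a one-shot warning sound through TimeDisplay near the end.
; Reaching the victory score or catching the Snitch wins, while timing out below target loses.
; Either ending switches the Broom's UI widget and freezes global time dilation.
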(event `self.ReceiveBeginPlay`
  (`self.Restart`))

(event `OnReset`
  (goto _label :!via `Reset`))

(event `self.ReceiveTick`
  (params (DeltaSeconds :type "Float (single-precision)"))
  (bind _asmain_game_state (cast `/Game/Blueprints/MainGameState` (`GameplayStatics.GetGameState`) :!pure true))
  (set `self.Delta` DeltaSeconds)
  (if (`/Game/Blueprints/MainGameState.IsGameRunning` _asmain_game_state)
    (bind _output_get (set `/Game/Blueprints/MainGameState.Timer` (- (`/Game/Blueprints/MainGameState.Timer` _asmain_game_state) (`self.Delta`)) _asmain_game_state))
    (if (> _output_get 0.0)
      (if (not (> _output_get 11.295))
        (`/Engine/EditorBlueprintResources/StandardMacros.DoOnce` false :!label _label
          (:`Completed`
            (`/Game/Pawns/TimeDisplay.PlayTimerEndSound` (`self.TimeDisplay`)))))
      (elif (>= (`/Game/Blueprints/MainGameState.Score` _asmain_game_state) (`/Game/Blueprints/MainGameInstance.VictoryScore` (cast `/Game/Blueprints/MainGameInstance` (`GameplayStatics.GetGameInstance`) :!pure true)))
        (`self.WinGame`)
        (else
          (`self.LooseGame`))))))

(fn `AddScore`
  (bind _asmain_game_state (cast `/Game/Blueprints/MainGameState` (`GameplayStatics.GetGameState`) :!pure true))
  (bind _output_get (set `/Game/Blueprints/MainGameState.Score` (+ (`/Game/Blueprints/MainGameState.Score` _asmain_game_state) 1) _asmain_game_state))
  (if (not (< _output_get (`/Game/Blueprints/MainGameInstance.VictoryScore` (cast `/Game/Blueprints/MainGameInstance` (`GameplayStatics.GetGameInstance`) :!pure true))))
    (`self.WinGame`)))

(fn `CatchSnitch`
  (`self.WinGame`))

(fn `LooseGame`
  (set `/Game/Blueprints/MainGameState.IsGameRunning` false (cast `/Game/Blueprints/MainGameState` (`GameplayStatics.GetGameState`) :!pure true))
  (`/Game/Widget/UIGame.SetGameUI` (cast `/Game/Widget/UIGame` (`WidgetComponent.GetUserWidgetObject` (`/Game/Pawns/Broom.Widget` (cast `/Game/Pawns/Broom` (`GameplayStatics.GetPlayerPawn` 0) :!pure true))) :!pure true) "NewEnumerator1")
  (`GameplayStatics.SetGlobalTimeDilation` 0.0))

(fn `Restart`
  (bind _asmain_game_state (cast `/Game/Blueprints/MainGameState` (`GameplayStatics.GetGameState`) :!pure true))
  (set `/Game/Blueprints/MainGameState.Timer` (`KismetMathLibrary.Conv_IntToDouble` (`/Game/Blueprints/MainGameInstance.MatchLength` (cast `/Game/Blueprints/MainGameInstance` (`GameplayStatics.GetGameInstance`) :!pure true))) _asmain_game_state)
  (set `/Game/Blueprints/MainGameState.Score` 0 _asmain_game_state)
  (set `/Game/Blueprints/MainGameState.IsGameRunning` true _asmain_game_state)
  (`self.OnReset`))

(fn `SetTimeDisplay`
  (params (TimeDisplay :type "/Game/Pawns/TimeDisplay Object Reference"))
  (set `self.TimeDisplay` TimeDisplay))

(fn `UserConstructionScript`)

(fn `WinGame`
  (bind _asmain_game_state (cast `/Game/Blueprints/MainGameState` (`GameplayStatics.GetGameState`) :!pure true))
  (if (`/Game/Blueprints/MainGameState.IsGameRunning` _asmain_game_state)
    (set `/Game/Blueprints/MainGameState.IsGameRunning` false _asmain_game_state)
    (`/Game/Pawns/TimeDisplay.PlayGameEndSound` (`self.TimeDisplay`))
    (`/Game/Widget/UIGame.SetGameUI` (cast `/Game/Widget/UIGame` (`WidgetComponent.GetUserWidgetObject` (`/Game/Pawns/Broom.Widget` (cast `/Game/Pawns/Broom` (`GameplayStatics.GetPlayerPawn` 0) :!pure true))) :!pure true) "NewEnumerator0")
    (`GameplayStatics.SetGlobalTimeDilation` 0.0)))